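; Base enemy pawn for PistolWhip that handles spawn and death dissolve, weapon equipping and hit score feedback.
; A timeline drives the mesh's Appearance material parameter on BeginPlay, equips the weapon once past a threshold while alive, and reverses after the parent Death logic.
; On a hit notification, it creates an animated score widget in the ScoreWidget component and rotates it to face the player pawn.
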(event `self.ReceiveBeginPlay`
  ;[0 0 0] Appearance and Dissolve
  (`MeshComponent.SetScalarParameterValueOnMaterials` (`self.Mesh`) "Appearance" 0.0)
  (bind (_direction _appearance) (`Timeline|Timeline_0` :!label _label)
    (:`Update`
      (`MeshComponent.SetScalarParameterValueOnMaterials` (`self.Mesh`) "Appearance" _appearance)
      (if (and (`self.bAlive`) (> _appearance 0.6))
        (`/Engine/EditorBlueprintResources/StandardMacros.DoOnce` false
          (:`Completed`
            (`self.EquipWeapon`)))))))

(event `self.Death`
  ;[0 0 0] Death Event
  (`parent.Death`)
  (goto _label :!via `Reverse`))

(event `self.NotifyEnemyHit`
  (params (HitScore :type Integer))
  ;[0 0 0] Notify Enemy Hit
  (`self.ShowScoreWidget` HitScore)
  (`self.RotateWidgetToPlayer`))

(fn `RotateWidgetToPlayer`
  (bind _scorewidget (`self.ScoreWidget`))
  (`SceneComponent.K2_SetWorldRotation` _scorewidget (`KismetMathLibrary.FindLookAtRotation` (`SceneComponent.K2_GetComponentLocation` _scorewidget) (`self.K2_GetActorLocation` (`GameplayStatics.GetPlayerPawn` 0))) false false))

(fn `ShowScoreWidget`
  (params (Score :type Integer))
  (bind _returnvalue (`|CreateWidget` "/Game/PistolWhip/UI/Widgets/WBP_HitScore.WBP_HitScore_C"))
  (`WidgetComponent.SetWidget` (`self.ScoreWidget`) _returnvalue)
  (`/Game/PistolWhip/UI/Widgets/WBP_HitScore.SetScore` _returnvalue (`local.Score`))
  (`UserWidget.PlayAnimation` _returnvalue (`/Game/PistolWhip/UI/Widgets/WBP_HitScore.Show` _returnvalue) 0.0 1 "Forward" 1.0 false)
  (return))

(fn `UserConstructionScript`)