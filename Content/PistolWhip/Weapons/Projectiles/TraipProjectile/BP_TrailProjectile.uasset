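; Pistol Whip projectile that draws a growing trail with four torus components spaced along it, pointing back toward its spawn location.
; Each tick it accumulates lifetime and derives the backward direction and a tail length that grows with lifetime up to a maximum.
; Those values set the Trail component's Target vector parameter to the tail end and reposition the toruses at offsets proportional to the current length.
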(event `self.ReceiveBeginPlay`
  (bind _output_get (set `self.InitialLocation` (`self.K2_GetActorLocation`)))
  (`FXSystemComponent.SetVectorParameter` (`self.Trail`) "Target" _output_get))

(event `self.ReceiveTick`
  (params (DeltaSeconds :type "Float (single-precision)"))
  (`self.Precalculate Data`)
  (`self.UpdateToruses`)
  (`self.Update Tail`))

(fn `CalculateMovementVector`
  (returns (ReturnValue :type "Vector Structure"))
  (return (`KismetMathLibrary.Normal` (- (`self.InitialLocation`) (`self.K2_GetActorLocation`)))))

(fn `CalculateTailLength`
  (returns (ReturnValue :type "Float (double-precision)"))
  (return (`KismetMathLibrary.FMin` (* (`self.BaseTailLength`) (`self.Lifetime`)) (`self.MaxTailLength`))))

(fn `Precalculate Data`
  (set `self.Lifetime` (+ (`GameplayStatics.GetWorldDeltaSeconds`) (`self.Lifetime`)))
  (set `self.MovementVector` (`self.CalculateMovementVector`))
  (set `self.TailLength` (`self.CalculateTailLength`)))

(fn `Update Tail`
  (`FXSystemComponent.SetVectorParameter` (`self.Trail`) "Target" (+ (`self.K2_GetActorLocation`) (* (`self.MovementVector`) (`self.TailLength`))))
  (return))

(fn `UpdateToruses`
  (`self.UpdateTorusLocation` (`self.Torus1`) 1)
  (`self.UpdateTorusLocation` (`self.Torus2`) 2)
  (`self.UpdateTorusLocation` (`self.Torus3`) 3)
  (`self.UpdateTorusLocation` (`self.Torus4`) 4))

(fn `UpdateTorusLocation`
  (params (Torus :type "StaticMeshComponent Object Reference") (TorusIndex :type Integer))
  (bind _taillength (`self.TailLength`))
  (`SceneComponent.K2_SetWorldLocation` Torus (+ (`self.K2_GetActorLocation`) (* (`self.MovementVector`) (+ (* TorusIndex (/ _taillength 5.0)) (/ _taillength 10.0)))) false false))

(fn `UserConstructionScript`)